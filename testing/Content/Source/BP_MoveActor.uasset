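; BP_MoveActor is an actor that slides its Cube component back and forth along its relative X axis.
; Pressing P toggles a fast looping timer that calls UpdateMove by function name, so movement runs without Tick.
; UpdateMove offsets the Cube by a Speed-scaled step and flips IsRight when it passes either end of a fixed range.
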(event `self.ReceiveBeginPlay`)

(event `self.ReceiveTick`
  (params (DeltaSeconds :type "Float (single-precision)")))

(event `/Game/Source/BPI_move.PressP`
  (if (`KismetSystemLibrary.K2_TimerExists` null "UpdateMove")
    (`KismetSystemLibrary.K2_ClearTimer` null "UpdateMove")
    (else
      (`KismetSystemLibrary.K2_SetTimer` null "UpdateMove" 0.01 true))))

(fn `UpdateMove`
  (bind _returnvalue (* 0.01 (`self.Speed`)))
  (bind _relativelocation_x (`KismetMathLibrary.BreakVector` (`SceneComponent.RelativeLocation` (`self.Cube`))))
  (bind _relativelocation_x_2 (`KismetMathLibrary.BreakVector` (`SceneComponent.RelativeLocation` (`self.Cube`))))
  (if (`self.isRight`)
    (`SceneComponent.K2_AddRelativeLocation` (`self.Cube`) (`KismetMathLibrary.MakeVector` _returnvalue) false false)
    (if (> _relativelocation_x_2 200.0)
      (set `self.isRight` false))
    (else
      (bind _result (`/Engine/EditorBlueprintResources/StandardMacros.NegateFloat` _returnvalue)
        (:`  `
          (`SceneComponent.K2_AddRelativeLocation` (`self.Cube`) (`KismetMathLibrary.MakeVector` _result) false false)
          (if (<= _relativelocation_x 0.0)
            (set `self.isRight` true)))))))

(fn `UserConstructionScript`)