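; Actor that moves its Cube component around a square path in relative X/Y space.
; While IsPlay is set, Tick switches on MoveType to run one of four directional functions, each advancing to the next at DesPosition or zero.
; Separately, PressP toggles a looping timer on UpdateMove, which ping-pongs the cube along X between fixed bounds using a fixed time step.
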(event `self.ReceiveBeginPlay`)

(event `self.ReceiveTick`
  (params (DeltaSeconds :type "Float (single-precision)"))
  (if (`self.IsPlay`)
    (switch `/Game/Source/EN_MoveType` (`self.MoveType`)
      (:`NewEnumerator0`
        (`self.MoveRight` DeltaSeconds))
      (:`NewEnumerator1`
        (`self.MoveLeft` DeltaSeconds))
      (:`NewEnumerator2`
        (`self.MoveUp` DeltaSeconds))
      (:`NewEnumerator3`
        (`self.MoveBottom` DeltaSeconds)))))

(event `/Game/Source/BPI_move.PressP`
  (if (`KismetSystemLibrary.K2_TimerExists` null "UpdateMove")
    (`KismetSystemLibrary.K2_ClearTimer` null "UpdateMove")
    (else
      (`KismetSystemLibrary.K2_SetTimer` null "UpdateMove" 0.01 true))))

(fn `MoveBottom`
  (params (DeltaSeceond :type "Float (double-precision)"))
  (bind (_relativelocation_x _relativelocation_y) (`KismetMathLibrary.BreakVector` (`SceneComponent.RelativeLocation` (`self.Cube`))))
  (bind _result (`/Engine/EditorBlueprintResources/StandardMacros.NegateFloat` (* DeltaSeceond (`self.Speed`)))
    (:`  `
      (`SceneComponent.K2_AddRelativeLocation` (`self.Cube`) (`KismetMathLibrary.MakeVector` 0.0 _result) false false)
      (if (< _relativelocation_y 0.0)
        (set `self.MoveType` "NewEnumerator0")))))

(fn `MoveLeft`
  (params (DeltaSeceond :type "Float (double-precision)"))
  (bind _relativelocation_x (`KismetMathLibrary.BreakVector` (`SceneComponent.RelativeLocation` (`self.Cube`))))
  (bind _result (`/Engine/EditorBlueprintResources/StandardMacros.NegateFloat` (* DeltaSeceond (`self.Speed`)))
    (:`  `
      (`SceneComponent.K2_AddRelativeLocation` (`self.Cube`) (`KismetMathLibrary.MakeVector` _result) false false)
      (if (< _relativelocation_x 0.0)
        (set `self.MoveType` "NewEnumerator3")))))

(fn `MoveRight`
  (params (DeltaSeceond :type "Float (double-precision)"))
  (bind _relativelocation_x (`KismetMathLibrary.BreakVector` (`SceneComponent.RelativeLocation` (`self.Cube`))))
  (`SceneComponent.K2_AddRelativeLocation` (`self.Cube`) (`KismetMathLibrary.MakeVector` (* DeltaSeceond (`self.Speed`))) false false)
  (if (> _relativelocation_x (`self.DesPosition`))
    (set `self.MoveType` "NewEnumerator2")))

(fn `MoveUp`
  (params (DeltaSeceond :type "Float (double-precision)"))
  (bind (_relativelocation_x _relativelocation_y) (`KismetMathLibrary.BreakVector` (`SceneComponent.RelativeLocation` (`self.Cube`))))
  (`SceneComponent.K2_AddRelativeLocation` (`self.Cube`) (`KismetMathLibrary.MakeVector` 0.0 (* DeltaSeceond (`self.Speed`))) false false)
  (if (> _relativelocation_y (`self.DesPosition`))
    (set `self.MoveType` "NewEnumerator1")))

(fn `UpdateMove`
  (bind _returnvalue (* 0.01 (`self.Speed`)))
  (bind _relativelocation_x (`KismetMathLibrary.BreakVector` (`SceneComponent.RelativeLocation` (`self.Cube`))))
  (bind _relativelocation_x_2 (`KismetMathLibrary.BreakVector` (`SceneComponent.RelativeLocation` (`self.Cube`))))
  (if (`self.isRight`)
    (`SceneComponent.K2_AddRelativeLocation` (`self.Cube`) (`KismetMathLibrary.MakeVector` _returnvalue) false false)
    (if (> _relativelocation_x_2 200.0)
      (set `self.isRight` false))
    (else
      (bind _result (`/Engine/EditorBlueprintResources/StandardMacros.NegateFloat` _returnvalue)
        (:`  `
          (`SceneComponent.K2_AddRelativeLocation` (`self.Cube`) (`KismetMathLibrary.MakeVector` _result) false false)
          (if (<= _relativelocation_x 0.0)
            (set `self.isRight` true)))))))

(fn `UserConstructionScript`)