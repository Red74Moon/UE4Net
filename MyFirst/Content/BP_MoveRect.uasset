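; Actor that moves its Sphere component around a square path in the relative XY plane, with the P key toggling movement on and off.
; While playing, Tick passes delta time to UpDateMoveRect, which switches on MoveType to run one of four direction functions.
; Each function moves the sphere by Speed along one axis and sets the next direction once it passes DestPos or zero, looping right, up, left, bottom.
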(event `self.ReceiveTick`
  (params (DeltaSeconds :type "Float (single-precision)"))
  (if (`self.IsPlay`)
    (`self.UpDateMoveRect` DeltaSeconds DeltaSeconds DeltaSeconds DeltaSeconds)))

(event `/Game/BPI_PressP.PressP`
  (set `self.IsPlay` (not (`self.IsPlay`))))

(fn `Move Left`
  (params (DeltaSecond :type "Float (double-precision)"))
  (bind _sphere (`self.Sphere`))
  (bind _relativelocation_x (`KismetMathLibrary.BreakVector` (`SceneComponent.RelativeLocation` _sphere)))
  (bind _result (`/Engine/EditorBlueprintResources/StandardMacros.NegateFloat` (* DeltaSecond (`self.Speed`)))
    (:`  `
      (`SceneComponent.K2_AddRelativeLocation` _sphere (`KismetMathLibrary.MakeVector` _result) false false)
      (if (< _relativelocation_x 0.0)
        (set `self.MoveType` "NewEnumerator3")))))

(fn `MoveBottom`
  (params (DeltaSeond :type "Float (double-precision)"))
  (bind (_relativelocation_x _relativelocation_y) (`KismetMathLibrary.BreakVector` (`SceneComponent.RelativeLocation` (`self.Sphere`))))
  (bind _result (`/Engine/EditorBlueprintResources/StandardMacros.NegateFloat` (* DeltaSeond (`self.Speed`)))
    (:`  `
      (`SceneComponent.K2_AddLocalOffset` (`self.Sphere`) (`KismetMathLibrary.MakeVector` 0.0 _result) false false)
      (if (< _relativelocation_y 0.0)
        (set `self.MoveType` "NewEnumerator0")))))

(fn `MoveRight`
  (params (DelteSecond :type "Float (double-precision)"))
  (bind _relativelocation_x (`KismetMathLibrary.BreakVector` (`SceneComponent.RelativeLocation` (`self.Sphere`))))
  (`SceneComponent.K2_AddRelativeLocation` (`self.Sphere`) (`KismetMathLibrary.MakeVector` (* DelteSecond (`self.Speed`))) false false)
  (if (> _relativelocation_x (`self.DestPos`))
    (set `self.MoveType` "NewEnumerator2")))

(fn `MoveUp`
  (params (DeltaSeond :type "Float (double-precision)"))
  (bind (_relativelocation_x _relativelocation_y) (`KismetMathLibrary.BreakVector` (`SceneComponent.RelativeLocation` (`self.Sphere`))))
  (`SceneComponent.K2_AddRelativeLocation` (`self.Sphere`) (`KismetMathLibrary.MakeVector` 0.0 (* DeltaSeond (`self.Speed`))) false false)
  (if (> _relativelocation_y (`self.DestPos`))
    (set `self.MoveType` "NewEnumerator1")))

(fn `UpDateMoveRect`
  (params (DelteSecond :type "Float (double-precision)") (DeltaSecond :type "Float (double-precision)") (DeltaSeond :type "Float (double-precision)") (DeltaSeond2 :type "Float (double-precision)"))
  (if (`self.IsPlay`)
    (switch `/Game/EN_MoveType` (`self.MoveType`)
      (:`NewEnumerator0`
        (`self.MoveRight` DelteSecond))
      (:`NewEnumerator1`
        (`self.Move Left` DeltaSecond))
      (:`NewEnumerator2`
        (`self.MoveUp` DeltaSeond))
      (:`NewEnumerator3`
        (`self.MoveBottom` DeltaSeond2)))))

(fn `UserConstructionScript`)