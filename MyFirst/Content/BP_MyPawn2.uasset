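; BP_MyPawn2 is a free-flying pawn with mouse look that offsets itself along camera axes without sweeping.
; Speed inputs adjust PlayerSpeed for forward and vertical movement, though slowing from the cap or below drops straight to minimum, and strafing uses a fixed speed.
; R and F nudge a referenced MoveActor up or down.
; At BeginPlay it caches actors implementing BPI_PressP, then messages them when P is pressed.
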(event `Key|R`
  (params (Key :type "Key Structure"))
  (:`Pressed`
    (`/Game/BP_MoveActor.MoveUp` (`self.MoveActor`) 0.01)))

(event `Key|F`
  (params (Key :type "Key Structure"))
  (:`Pressed`
    (`/Game/BP_MoveActor.MoveDown` (`self.MoveActor`) 0.01)))

(event `InputAction|SpeedUp`
  (params (Key :type "Key Structure"))
  ;[1 1 1] 1-speedup, 2-speeddown
  (:`Pressed`
    (bind _output_get (set `self.PlayerSpeed` (+ (`self.PlayerSpeed`) 10.0)))
    (if (> _output_get 100.0)
      (set `self.PlayerSpeed` 100.0))))

(event `InputAction|SpeedDown`
  (params (Key :type "Key Structure"))
  ;[1 1 1] 1-speedup, 2-speeddown
  (:`Pressed`
    (bind _output_get (set `self.PlayerSpeed` (- (`self.PlayerSpeed`) 10.0)))
    (if (<= _output_get 100.0)
      (set `self.PlayerSpeed` 10.0))))

(event `InputAxis|MoveUp`
  (params (AxisValue :type "Float (single-precision)"))
  ;[1 1 1] 4방향 및 위아래, 마우스 움직임
  (`self.K2_AddActorWorldOffset` (* (`self.GetActorUpVector` (`GameplayStatics.GetPlayerCameraManager` 0)) (* AxisValue (`self.PlayerSpeed`)))))

(event `self.ReceiveBeginPlay`
  ;[1 1 1] 코멘트
  (bind _outactors (`GameplayStatics.GetAllActorsOfClass` "/Script/Engine.Actor"))
  (for _array_element _outactors
    (if (`KismetSystemLibrary.DoesImplementInterface` _array_element "/Game/BPI_PressP.BPI_PressP_C")
      (`KismetArrayLibrary.Array_Add` (`self.Actors`) _array_element))))

(event `InputAxis|MoveForward`
  (params (AxisValue :type "Float (single-precision)"))
  ;[1 1 1] 4방향 및 위아래, 마우스 움직임
  (`self.K2_AddActorWorldOffset` (* (`self.GetActorForwardVector` (`GameplayStatics.GetPlayerCameraManager` 0)) (* AxisValue (`self.PlayerSpeed`)))))

(event `InputAxis|MoveRight`
  (params (AxisValue :type "Float (single-precision)"))
  ;[1 1 1] 4방향 및 위아래, 마우스 움직임
  (`self.K2_AddActorWorldOffset` (* (`self.GetActorRightVector` (`GameplayStatics.GetPlayerCameraManager` 0)) (* AxisValue 10.0))))

(event `Key|P`
  (params (Key :type "Key Structure"))
  ;[1 1 1] 코멘트
  (:`Pressed`
    (for _array_element (`self.Actors`)
      (if (`KismetSystemLibrary.DoesImplementInterface` _array_element "/Game/BPI_PressP.BPI_PressP_C")
        (message `/Game/BPI_PressP.PressP` _array_element)))))

(event `InputAxis|LookRight`
  (params (AxisValue :type "Float (single-precision)"))
  ;[1 1 1] 4방향 및 위아래, 마우스 움직임
  (`self.AddControllerYawInput` AxisValue))

(event `InputAxis|LookUp`
  (params (AxisValue :type "Float (single-precision)"))
  ;[1 1 1] 4방향 및 위아래, 마우스 움직임
  (`self.AddControllerPitchInput` AxisValue))

(fn `UserConstructionScript`)