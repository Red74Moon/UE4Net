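; Player pawn that flies freely relative to the camera and acts as a controller for four demo actors it spawns on BeginPlay.
; Input axes drive look and movement; PlayerSpeed scales forward and vertical motion, while strafing uses a fixed speed.
; Speed-up raises PlayerSpeed in capped steps, but speed-down's clamp snaps it straight to the minimum.
; R/F nudge MoveActor up or down, and P toggles or signals play state on all four actors.
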(event `Key|R`
  (params (Key :type "Key Structure"))
  (:`Pressed`
    (`/Game/BP_MoveActor.MoveUp` (`self.MoveActor`) 0.01)))

(event `Key|F`
  (params (Key :type "Key Structure"))
  (:`Pressed`
    (`/Game/BP_MoveActor.MoveDown` (`self.MoveActor`) 0.01)))

(event `InputAction|SpeedUp`
  (params (Key :type "Key Structure"))
  ;[1 1 1] 1-speedup, 2-speeddown
  (:`Pressed`
    (bind _output_get (set `self.PlayerSpeed` (+ (`self.PlayerSpeed`) 10.0)))
    (if (> _output_get 100.0)
      (set `self.PlayerSpeed` 100.0))))

(event `InputAction|SpeedDown`
  (params (Key :type "Key Structure"))
  ;[1 1 1] 1-speedup, 2-speeddown
  (:`Pressed`
    (bind _output_get (set `self.PlayerSpeed` (- (`self.PlayerSpeed`) 10.0)))
    (if (<= _output_get 100.0)
      (set `self.PlayerSpeed` 10.0))))

(event `self.ReceiveBeginPlay`
  (`|ExecutionSequence`
    (:`then_0`
      (bind _returnvalue (`|SpawnActorFromClass` "/Game/BP_MoveActor.BP_MoveActor_C" (`KismetMathLibrary.MakeTransform` (100.0 0.0 0.0)) "Undefined" "OverrideRootScale" null null))
      (set `self.MoveActor` _returnvalue))
    (:`then_1`
      (bind _returnvalue_2 (`|SpawnActorFromClass` "/Game/BP_MoveRect.BP_MoveRect_C" (`KismetMathLibrary.MakeTransform` (0.0 0.0 0.0)) "Undefined" "OverrideRootScale" null null))
      (set `self.MoveRect` _returnvalue_2))
    (:`then_2`
      (bind _returnvalue_3 (`|SpawnActorFromClass` "/Game/BP_RotationBall.BP_RotationBall_C" (`KismetMathLibrary.MakeTransform` (0.0 0.0 100.0)) "Undefined" "OverrideRootScale" null null))
      (set `self.RotationBall` _returnvalue_3))
    (:`then_3`
      (bind _returnvalue_4 (`|SpawnActorFromClass` "/Game/BP_TimeLineActor.BP_TimeLineActor_C" (`KismetMathLibrary.MakeTransform` (0.0 0.0 0.0)) "Undefined" "OverrideRootScale" null null))
      (set `self.TimeLineActor` _returnvalue_4))))

(event `InputAxis|MoveUp`
  (params (AxisValue :type "Float (single-precision)"))
  ;[1 1 1] 4방향 및 위아래, 마우스 움직임
  (`self.K2_AddActorWorldOffset` (* (`self.GetActorUpVector` (`GameplayStatics.GetPlayerCameraManager` 0)) (* AxisValue (`self.PlayerSpeed`)))))

(event `InputAxis|MoveForward`
  (params (AxisValue :type "Float (single-precision)"))
  ;[1 1 1] 4방향 및 위아래, 마우스 움직임
  (`self.K2_AddActorWorldOffset` (* (`self.GetActorForwardVector` (`GameplayStatics.GetPlayerCameraManager` 0)) (* AxisValue (`self.PlayerSpeed`)))))

(event `Key|P`
  (params (Key :type "Key Structure"))
  (bind _moverect (`self.MoveRect`))
  (bind _moveactor (`self.MoveActor`))
  (:`Pressed`
    (`/Game/BP_RotationBall.PressP` (`self.RotationBall`))
    (`/Game/BP_TimeLineActor.PressP` (`self.TimeLineActor`))
    (set `/Game/BP_MoveRect.IsPlay` (not (`/Game/BP_MoveRect.IsPlay` _moverect)) _moverect)
    (set `/Game/BP_MoveActor.IsPlay` (not (`/Game/BP_MoveActor.IsPlay` _moveactor)) _moveactor)))

(event `InputAxis|MoveRight`
  (params (AxisValue :type "Float (single-precision)"))
  ;[1 1 1] 4방향 및 위아래, 마우스 움직임
  (`self.K2_AddActorWorldOffset` (* (`self.GetActorRightVector` (`GameplayStatics.GetPlayerCameraManager` 0)) (* AxisValue 10.0))))

(event `InputAxis|LookRight`
  (params (AxisValue :type "Float (single-precision)"))
  ;[1 1 1] 4방향 및 위아래, 마우스 움직임
  (`self.AddControllerYawInput` AxisValue))

(event `InputAxis|LookUp`
  (params (AxisValue :type "Float (single-precision)"))
  ;[1 1 1] 4방향 및 위아래, 마우스 움직임
  (`self.AddControllerPitchInput` AxisValue))

(fn `UserConstructionScript`)