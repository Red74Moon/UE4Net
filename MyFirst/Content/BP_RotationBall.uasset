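; BP_RotationBall is an actor that swings its Center component back and forth on roll, toggled by the P key.
; A timeline scales its value by 45 degrees to set the roll, flipping IsRight on finish to alternate between Play and Reverse.
; Stopping halts the timeline and clears IsPlay.
; An uncalled UpdateAddRotation function holds an incremental, speed-based version that reverses at ±45 degrees.
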(event `self.ReceiveTick`
  (params (DeltaSeconds :type "Float (single-precision)")))

(event `/Game/BPI_PressP.PressP`
  (if (`self.IsPlay`)
    (`self.StopRotatoinBall`)
    (else
      (`self.StartRotationBall`))))

(event `self.ReceiveBeginPlay`)

(event `StartRotationBall`
  (set `self.IsPlay` true)
  (if (`self.IsRight`) :!label _label
    (bind (_direction _value) (`Timeline|타임라인_0` :!label _label_2)
      (:`Update`
        (`SceneComponent.K2_SetRelativeRotation` (`self.Center`) (`KismetMathLibrary.MakeRotator` (* _value 45.0)) false false))
      (:`Finished`
        (set `self.IsRight` (not (`self.IsRight`)))
        (goto _label)))
    (else
      (goto _label_2 :!via `Reverse`))))

(event `StopRotatoinBall`
  (set `self.IsPlay` false)
  (goto _label_2 :!via `Stop`))

(fn `UpdateAddRotation`
  (params (A :type "Float (double-precision)"))
  (bind _center (`self.Center`))
  (bind _returnvalue (* A (`self.Speed`)))
  (bind _relativerotation_roll (`KismetMathLibrary.BreakRotator` (`SceneComponent.RelativeRotation` _center)))
  (bind _relativerotation_roll_2 (`KismetMathLibrary.BreakRotator` (`SceneComponent.RelativeRotation` _center)))
  (if (`self.IsRight`)
    (`SceneComponent.K2_AddRelativeRotation` _center (`KismetMathLibrary.MakeRotator` _returnvalue) false false)
    (if (> _relativerotation_roll 45.0)
      (set `self.IsRight` false))
    (else
      (bind _result (`/Engine/EditorBlueprintResources/StandardMacros.NegateFloat` _returnvalue)
        (:`  `
          (`SceneComponent.K2_AddRelativeRotation` _center (`KismetMathLibrary.MakeRotator` _result) false false)
          (if (< _relativerotation_roll_2 -45.0)
            (set `self.IsRight` true)))))))

(fn `UserConstructionScript`)