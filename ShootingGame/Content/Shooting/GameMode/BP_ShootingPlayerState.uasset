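; Player state for the shooting game that holds a player's HP and broadcasts its changes to listeners.
; AddDamage subtracts damage within a 0–100 clamp and is called with zero on BeginPlay.
; OnRep_HP logs the value and fires an UpdateHp dispatcher, plus an UpdateHUD dispatcher only when this state belongs to player controller 0.
; The dispatcher replaces a direct HUD cast, which remains as unreachable nodes.
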(event `self.ReceiveBeginPlay`
  (`self.AddDamage` 0.0))

(fn `AddDamage`
  (params (Damage :type "Float (double-precision)"))
  (if true
    (set `self.HP` (`KismetMathLibrary.FClamp` (- (`self.HP`) Damage) 0.0 100.0))))

(fn `OnRep_HP`
  (`KismetSystemLibrary.PrintString` (`KismetStringLibrary.Concat_StrStr` "OnRepHp CurHP : " (`KismetStringLibrary.Conv_DoubleToString` (`self.HP`))) false true (struct :`G` 0.66 :`B` 1.0 :`A` 1.0) 20.0)
  (`self.EventDispatcher_UpdateHp` (`self.HP`) 100.0)
  ;[1 1 1] 나만 업데이트하기 위해서
  (if (== self (`Controller.PlayerState` (`GameplayStatics.GetPlayerController` 0)))
    (`self.EventDispatcher_UpdateHUD` (`self.HP`) 100.0)))

(fn `UserConstructionScript`)