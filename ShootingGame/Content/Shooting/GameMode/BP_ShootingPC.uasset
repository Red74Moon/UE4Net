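; BP_ShootingPC is the shooting mode's player controller, passing the player's locally stored name to the server when it possesses a pawn.
; The server-side Possess event calls ResClientPossess on the client, which reads Name from ShootingGameInstance.
; The client sends it back through ReqSetNewName, where the server applies it with SetName on BP_ShootingPlayerState.
; Debug prints trace each step.
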(event `self.ReceivePossess`
  (params (PossessedPawn :type "Pawn Object Reference"))
  ;[1 0 0] Possess 실행(서버에서 실행) 빙의 이벤트
  (`KismetSystemLibrary.PrintString` (`KismetStringLibrary.Concat_StrStr` "On Possessed : " (`KismetSystemLibrary.GetDisplayName` PossessedPawn)) false true (struct :`G` 0.66 :`B` 1.0 :`A` 1.0) 60.0)
  (`self.ResClientPossess`))

(event `ResClientPossess`
  ;[1 1 1] 커스텀함수(클라이언트에서 서버에 접속됨을 알수 있다.) 빙의이벤트 수신
  (`KismetSystemLibrary.PrintString` (`KismetStringLibrary.Concat_StrStr` "ResClientPossess : " (`KismetSystemLibrary.GetDisplayName` self)) false true (struct :`G` 0.66 :`B` 1.0 :`A` 1.0) 60.0)
  (bind _asshooting_game_instance (cast `/Game/Shooting/GameMode/ShootingGameInstance` (`GameplayStatics.GetGameInstance`)))
  (`self.ReqSetNewName` (`/Game/Shooting/GameMode/ShootingGameInstance.Name` _asshooting_game_instance)))

(event `ReqSetNewName`
  (params (NewName :type String))
  ;[1 0 0] (Server)새로운 이름 적용
  (`KismetSystemLibrary.PrintString` "ReqSetNewName : " false true (struct :`R` 1.0 :`A` 1.0) 60.0)
  (bind _asbp_shooting_player_state (cast `/Game/Shooting/GameMode/BP_ShootingPlayerState` (`self.PlayerState`)))
  (`/Game/Shooting/GameMode/BP_ShootingPlayerState.SetName` _asbp_shooting_player_state NewName))

(fn `UserConstructionScript`)