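; HUD Blueprint for the shooting game that creates the main shooting widget and sets game-only input with the cursor hidden.
; Its functions forward HP, ammo and pickup-guide position updates to that widget.
; It binds to the player state's HP update dispatcher, retrying on a timer until the cast succeeds.
; Weapon-name text targets a separate widget whose creation code is disconnected and never runs.
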(event `self.ReceiveBeginPlay`
  (bind _returnvalue (`GameplayStatics.GetPlayerController` 0))
  (`|ExecutionSequence`
    (:`then_0`
      (bind _returnvalue_2 (`|CreateWidget` "/Game/Shooting/Widget/ShootingHUDWidget.ShootingHUDWidget_C"))
      (bind _output_get (set `self.ShootingHudWidget` _returnvalue_2))
      (`UserWidget.AddToViewport` _output_get 0)
      (`self.UpdateBindPlayerState`)
      (`WidgetBlueprintLibrary.SetInputMode_GameOnly` _returnvalue)
      (set `PlayerController.bShowMouseCursor` false _returnvalue))))

(fn `HidePickUpGuide`
  (`/Game/Shooting/Widget/ShootingHUDWidget.HideGuidePostion` (`self.ShootingHudWidget`)))

(fn `Set Hp Text`
  (params (HP :type "Float (double-precision)"))
  (`/Game/Shooting/Widget/ShootingHUDWidget.SetHpText` (`self.ShootingHudWidget`) HP))

(fn `Set Weapon Name Text`
  (params (WeaponName :type String))
  (`KismetSystemLibrary.PrintString` WeaponName false true (struct :`R` 1.0 :`G` 0.020309 :`B` 0.010362 :`A` 1.0) 20.0)
  (`/Game/Shooting/Widget/WeaponNameHUDWidget.SetWeaponName_hudwidget` (`self.WeaponNameHudWidget`) WeaponName))

(fn `SetAmmoText`
  (params (Ammo :type Integer))
  (`/Game/Shooting/Widget/ShootingHUDWidget.SetAmmoText` (`self.ShootingHudWidget`) Ammo))

(fn `SetHp`
  (params (CurHP :type "Float (double-precision)") (MaxHP :type "Float (double-precision)"))
  (`/Game/Shooting/Widget/ShootingHUDWidget.SetHP` (`self.ShootingHudWidget`) CurHP MaxHP))

(fn `UpdateBindPlayerState`
  (bind _asbp_shooting_player_state (cast `/Game/Shooting/GameMode/BP_ShootingPlayerState` (`Controller.PlayerState` (`GameplayStatics.GetPlayerController` 0)))
    (:`then`
      (add `/Game/Shooting/GameMode/BP_ShootingPlayerState.EventDispatcher_UpdateHp` _asbp_shooting_player_state (`|CreateDelegate` :!event `SetHp`)))
    (:`CastFailed`
      (`KismetSystemLibrary.K2_SetTimer` null "UpdateBindPlayerState" 0.1))))

(fn `UpdatePickUpGuidePosition`
  (params (WorldLocation :type "Vector Structure"))
  (`/Game/Shooting/Widget/ShootingHUDWidget.UpdateGuidePostion` (`self.ShootingHudWidget`) WorldLocation))

(fn `UserConstructionScript`)