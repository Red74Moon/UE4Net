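; Data-driven pickup weapon that characters carry on a mesh socket, fire, reload and drop, with HUD pickup guide and ammo count.
; BeginPlay loads mesh, socket and ammo from DT_Weapon.
; PullTrigger checks ammo, plays the shoot montage and decrements the count, while separate DoShoot and DoReload perform the effects and refill.
; DoShoot line-traces from the camera only for the local owner, sending hits to ReqApplyDamage, logged as server-side.
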(event `self.ReceiveBeginPlay`
  (`self.Initialize`))

(event `/Game/Shooting/Data/BPI_Weapon.ShowPickUpGuide`
  (`KismetSystemLibrary.K2_SetTimer` null "UpdatePickupGuide" 0.001 true))

(event `self.ReceiveTick`
  (params (DeltaSeconds :type "Float (single-precision)")))

(event `self.PickUpCollision.OnComponentEndOverlap`
  (params (OverlappedComponent :type "PrimitiveComponent Object Reference") (OtherActor :type "Actor Object Reference") (OtherComp :type "PrimitiveComponent Object Reference") (OtherBodyIndex :type Integer))
  (`KismetSystemLibrary.K2_ClearTimer` null "UpdatePickupGuide")
  (bind _asbp_shooting_hud (cast `/Game/Shooting/HUD/BP_ShootingHUD` (`PlayerController.GetHUD` (`GameplayStatics.GetPlayerController` 0))))
  (`/Game/Shooting/HUD/BP_ShootingHUD.HidePickUpGuide` _asbp_shooting_hud))

(event `ReqApplyDamage`
  (params (DamagedActor :type "Actor Object Reference (by ref)") (BaseDamage :type "Float (double-precision)") (EventInstigator :type "Controller Object Reference (by ref)") (DamageCauser :type "Actor Object Reference (by ref)"))
  (`GameplayStatics.ApplyDamage` DamagedActor BaseDamage EventInstigator DamageCauser)
  (`KismetSystemLibrary.PrintString` (`KismetStringLibrary.Concat_StrStr` "(server) Apply Damage - " (`KismetSystemLibrary.GetDisplayName` DamagedActor)) false true (struct :`R` 1.0 :`A` 1.0) 20.0))

(fn `AttachToChar`
  (params (Characrter :type "Character Object Reference"))
  (returns (Result :type Boolean))
  (bind _static_mesh (`self.static mesh`))
  (bind _output_get (set `self.OwnChar` Characrter))
  (bind _asbp_shooting_hud (cast `/Game/Shooting/HUD/BP_ShootingHUD` (`PlayerController.GetHUD` (`GameplayStatics.GetPlayerController` 0))))
  (`/Game/Shooting/HUD/BP_ShootingHUD.SetAmmoText` _asbp_shooting_hud (`self.CurAmmo`))
  (`PrimitiveComponent.SetSimulatePhysics` _static_mesh false)
  (`PrimitiveComponent.SetCollisionEnabled` _static_mesh "NoCollision")
  (`PrimitiveComponent.SetCollisionEnabled` (`self.PickupCollision`) "NoCollision")
  (bind _returnvalue (`SceneComponent.K2_AttachToComponent` _static_mesh (`Character.Mesh` _output_get) (`self.Socket Name`) "SnapToTarget" "SnapToTarget" "KeepWorld" true))
  (return _returnvalue))

(fn `Check Shootable`
  (returns (Shootable :type Boolean))
  (`/Engine/EditorBlueprintResources/StandardMacros.IsValid` (`self.OwnChar`)
    (:`Is Valid`
      (if (> (`self.CurAmmo`) 0)
        (return true)
        (else
          (return false))))
    (:`Is Not Valid`
      (return false))))

(fn `DetachToChar`
  (params (Character :type "Character Object Reference"))
  (returns (Result :type Boolean))
  (bind _static_mesh (`self.static mesh`))
  (set `self.OwnChar` null)
  (`PrimitiveComponent.SetCollisionEnabled` _static_mesh "QueryAndPhysics")
  (`PrimitiveComponent.SetSimulatePhysics` _static_mesh true)
  (`SceneComponent.K2_DetachFromComponent` _static_mesh "KeepWorld" "KeepWorld" "KeepWorld" true)
  (return true))

(fn `DoReload`
  (params (Character :type "Character Object Reference"))
  (returns (Result :type Boolean))
  (bind _output_get (set `self.CurAmmo` (`.Ammo_10_5D6BAFFE44FFDBD13B6694990A0BCADB` (break `/Game/Shooting/Data/ST_Weapon` (`self.WeaponData`)))))
  (bind _asbp_shooting_hud (cast `/Game/Shooting/HUD/BP_ShootingHUD` (`PlayerController.GetHUD` (`GameplayStatics.GetPlayerController` 0))))
  (`/Game/Shooting/HUD/BP_ShootingHUD.SetAmmoText` _asbp_shooting_hud _output_get)
  (return true))

(fn `DoShoot`
  (params (Character :type "Character Object Reference"))
  (returns (Result :type Boolean))
  (bind _returnvalue (`GameplayStatics.GetPlayerCameraManager` 0))
  (bind _audio (`self.Audio`))
  (bind _returnvalue_2 (`self.K2_GetActorLocation` _returnvalue))
  (`AudioComponent.SetSound` _audio (`.ShootSound_5_EE39D85C4639EF727A4CF78DD5A5523E` (break `/Game/Shooting/Data/ST_Weapon` (`self.WeaponData`))))
  (`AudioComponent.Play` _audio 0.0)
  (`GameplayStatics.SpawnEmitterAtLocation` "/Game/StarterContent/Particles/P_Explosion.P_Explosion" (`SceneComponent.GetSocketLocation` (`self.static mesh`) "Muzzle") (struct) (0.1 0.1 0.1))
  ;[1 1 1] 나일때만(예외처리), 소유자만
  (if (== (`GameplayStatics.GetPlayerPawn` 0) (`self.OwnChar`))
    ;[1 1 1] 히트체크
    (bind (_outhit _returnvalue_3) (`KismetSystemLibrary.LineTraceSingleForObjects` :`Start` (+ _returnvalue_2 (* (`self.GetActorForwardVector` _returnvalue) 250.0)) :`End` (+ _returnvalue_2 (* (`self.GetActorForwardVector` _returnvalue) 2000.0)) :`ObjectTypes` (`|MakeArray` "ObjectTypeQuery1" "ObjectTypeQuery2" "ObjectTypeQuery3" "ObjectTypeQuery4" "ObjectTypeQuery6" :!type "EObjectTypeQuery Enum") :`DrawDebugType` "Persistent"))
    (if _returnvalue_3
      (`KismetSystemLibrary.PrintString` "(Client) ReqApplyDamage" false true (struct :`G` 0.66 :`B` 1.0 :`A` 1.0) 20.0)
      (`self.ReqApplyDamage` (`.HitActor` (`GameplayStatics.BreakHitResult` _outhit)) 10.0 (`Pawn.GetController` (`self.OwnChar`)) self)
      (return true))))

(fn `Initialize`
  (bind _returnvalue (`|GetDataTableRow` "/Game/Shooting/Data/DT_Weapon.DT_Weapon" (`self.ViewWeaponName`))
    (:`then`
      (bind _output_get (set `self.WeaponData` _returnvalue))
      (`|ExecutionSequence`
        (:`then_0`
          (bind (_staticmesh _socketname _shootsound _reloadsound _ammo) (break `/Game/Shooting/Data/ST_Weapon` _output_get))
          (`StaticMeshComponent.SetStaticMesh` (`self.static mesh`) _staticmesh))
        (:`then_1`
          (set `self.Socket Name` _socketname))
        (:`then_2`
          (set `self.CurAmmo` _ammo))))))

(fn `PlayReloadAnim`
  (params (Character :type "Character Object Reference"))
  (returns (Result :type Boolean))
  (bind _ownchar (`self.OwnChar`))
  (bind (_staticmesh _socketname _shootsound _reloadsound _ammo _shootmontage _shootmontageplayrate _reloadmontage _reloadmontageplayrate) (break `/Game/Shooting/Data/ST_Weapon` (`self.WeaponData`)))
  (`/Engine/EditorBlueprintResources/StandardMacros.IsValid` _ownchar
    (:`Is Valid`
      (`AnimInstance.Montage_Play` (`SkeletalMeshComponent.GetAnimInstance` (`Character.Mesh` _ownchar)) _reloadmontage _reloadmontageplayrate "MontageLength" 0.0 true)
      (return false))))

(fn `PlayShootMontage`
  (bind _ownchar (`self.OwnChar`))
  (bind (_staticmesh _socketname _shootsound _reloadsound _ammo _shootmontage _shootmontageplayrate) (break `/Game/Shooting/Data/ST_Weapon` (`self.WeaponData`)))
  (bind _shootable (`self.Check Shootable`))
  (if _shootable
    (`/Engine/EditorBlueprintResources/StandardMacros.IsValid` _ownchar
      (:`Is Valid`
        (`AnimInstance.Montage_Play` (`SkeletalMeshComponent.GetAnimInstance` (`Character.Mesh` _ownchar)) _shootmontage _shootmontageplayrate "MontageLength" 0.0 true)
        (bind _result (`/Engine/EditorBlueprintResources/StandardMacros.DecrementInt` (`self.CurAmmo`))
          (:`  `
            (bind _asbp_shooting_hud (cast `/Game/Shooting/HUD/BP_ShootingHUD` (`PlayerController.GetHUD` (`GameplayStatics.GetPlayerController` 0))))
            (`/Game/Shooting/HUD/BP_ShootingHUD.SetAmmoText` _asbp_shooting_hud _result)))))))

(fn `PullTrigger`
  (params (Character :type "Character Object Reference"))
  (returns (Result :type Boolean))
  (`self.PlayShootMontage`)
  (return true))

(fn `ReleaseTrigger`
  (params (Character :type "Character Object Reference"))
  (returns (Result :type Boolean))
  (return false))

(fn `Shoot`
  (`AudioComponent.Play` (`self.Audio`) 0.0)
  (`GameplayStatics.SpawnEmitterAtLocation` "/Game/StarterContent/Particles/P_Explosion.P_Explosion" (`SceneComponent.GetSocketLocation` (`self.static mesh`) "Muzzle") (struct) (0.1 0.1 0.1)))

(fn `UpdatePickupGuide`
  (bind _asbp_shooting_hud (cast `/Game/Shooting/HUD/BP_ShootingHUD` (`PlayerController.GetHUD` (`GameplayStatics.GetPlayerController` 0))))
  (`/Game/Shooting/HUD/BP_ShootingHUD.UpdatePickUpGuidePosition` _asbp_shooting_hud (`self.K2_GetActorLocation`)))

(fn `UserConstructionScript`)