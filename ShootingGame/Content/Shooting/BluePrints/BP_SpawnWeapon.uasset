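; BP_SpawnWeapon is an overlap-triggered spawner that creates a random weapon at its own location.
; Its OnActorOverlap override calls the parent, then on the server spawns a BP_MachineGun with ViewWeaponName set to a random row name from DT_Weapon.
; An unconnected branch would scatter several such weapons at random navigable points around the actor, but it never runs.
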(event `self.ReceiveActorBeginOverlap`
  (params (OtherActor :type "Actor Object Reference"))
  (`parent.ReceiveActorBeginOverlap` OtherActor))

(fn `OnActorOverlap`
  (params (OtherActor :type "Actor Object Reference"))
  (`parent.OnActorOverlap` null)
  (`/Engine/EditorBlueprintResources/ActorMacros.Switch Has Authority`
    (:`Authority`
      (bind _outrownames (`DataTableFunctionLibrary.GetDataTableRowNames` "/Game/Shooting/Data/DT_Weapon.DT_Weapon"))
      (`|SpawnActorFromClass` "/Game/Shooting/BluePrints/BP_MachineGun.BP_MachineGun_C" (`KismetMathLibrary.MakeTransform` (`self.K2_GetActorLocation`)) "Undefined" "OverrideRootScale" null (`|GetArrayItem` _outrownames (`KismetMathLibrary.RandomInteger` (`KismetArrayLibrary.Array_Length` _outrownames))) "Weapon1" null))))

(fn `UserConstructionScript`
  (`parent.UserConstructionScript`))