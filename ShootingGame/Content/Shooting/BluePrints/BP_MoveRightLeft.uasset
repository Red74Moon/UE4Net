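; BP_MoveRightLeft is an actor whose Cube component slides back and forth along its X axis.
; The PressP interface event toggles a fast looping timer that calls UpdateMoveRightLeft, so movement can start and stop without Tick.
; Each update offsets the cube by a Speed-scaled step and flips IsRight at fixed relative X limits, using AddRelativeLocation one way and AddLocalOffset the other.
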(event `self.ReceiveBeginPlay`
  ;[1 1 1] 코멘트
)

(event `/Game/Shooting/Data/BPI_MoveActor.PressP`
  ;[1 1 1] Interface Press P Event
  (if (`KismetSystemLibrary.K2_TimerExists` null "UpdateMoveRightLeft")
    (`KismetSystemLibrary.K2_ClearTimer` null "UpdateMoveRightLeft")
    (else
      (`KismetSystemLibrary.K2_SetTimer` null "UpdateMoveRightLeft" 0.01 true))))

(fn `UpdateMoveRightLeft`
  (bind _returnvalue (* 0.01 (`self.Speed`)))
  (bind _relativelocation_x (`KismetMathLibrary.BreakVector` (`SceneComponent.RelativeLocation` (`self.Cube`))))
  (bind _relativelocation_x_2 (`KismetMathLibrary.BreakVector` (`SceneComponent.RelativeLocation` (`self.Cube`))))
  (if (`self.Is Right`)
    ;[1 1 1] right
    (`SceneComponent.K2_AddRelativeLocation` (`self.Cube`) (`KismetMathLibrary.MakeVector` _returnvalue) false false)
    (if (> _relativelocation_x 200.0)
      (set `self.Is Right` false))
    (else
      ;[1 1 1] left
      (bind _result (`/Engine/EditorBlueprintResources/StandardMacros.NegateFloat` _returnvalue)
        (:`  `
          (`SceneComponent.K2_AddLocalOffset` (`self.Cube`) (`KismetMathLibrary.MakeVector` _result) false false)
          (if (< _relativelocation_x_2 -200.0)
            (set `self.Is Right` true)))))))

(fn `UserConstructionScript`)