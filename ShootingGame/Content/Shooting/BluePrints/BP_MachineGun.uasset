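; BP_MachineGun is a weapon Blueprint that provides automatic fire while the trigger is held.
; PullTrigger starts a looping timer that calls PlayShootMontage every tenth of a second, and ReleaseTrigger clears it.
; Each call plays the single-shot rifle montage, sped up, on the owning character's mesh if that character is valid.
; The Blueprint itself contains no projectile, trace or damage logic.
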(event `self.ReceiveBeginPlay`)

(fn `PlayShootMontage`
  (bind _ownchar (`self.OwnChar`))
  (`/Engine/EditorBlueprintResources/StandardMacros.IsValid` _ownchar
    (:`Is Valid`
      (`AnimInstance.Montage_Play` (`SkeletalMeshComponent.GetAnimInstance` (`Character.Mesh` _ownchar)) "/Game/Mannequin/Animations/InPlace/Rifle_ShootOnce_Montage.Rifle_ShootOnce_Montage" 1.5 "MontageLength" 0.0 true))))

(fn `PullTrigger`
  (params (Character :type "Character Object Reference"))
  (returns (Result :type Boolean))
  (`KismetSystemLibrary.K2_SetTimer` null "PlayShootMontage" 0.1 true)
  (return false))

(fn `ReleaseTrigger`
  (params (Character :type "Character Object Reference"))
  (returns (Result :type Boolean))
  (`KismetSystemLibrary.K2_ClearTimer` null "PlayShootMontage")
  (return false))

(fn `UserConstructionScript`
  (`parent.UserConstructionScript`))