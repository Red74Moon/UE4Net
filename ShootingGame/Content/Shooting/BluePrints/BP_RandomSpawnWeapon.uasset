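; BP_RandomSpawnWeapon is a spawner that places randomly chosen weapon pickups near its own location when play begins.
; On the authority only, a short loop spawns BP_MachineGun actors at random navigable points within a small radius.
; Each spawn receives a random DT_Weapon row name as ViewWeaponName, so one actor class covers whichever weapon row is picked.
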(event `self.ReceiveBeginPlay`
  (`/Engine/EditorBlueprintResources/ActorMacros.Switch Has Authority`
    (:`Authority`
      (for _ (range 2)
        (bind _outrownames (`DataTableFunctionLibrary.GetDataTableRowNames` "/Game/Shooting/Data/DT_Weapon.DT_Weapon"))
        (`|SpawnActorFromClass` "/Game/Shooting/BluePrints/BP_MachineGun.BP_MachineGun_C" (`KismetMathLibrary.MakeTransform` (`NavigationSystemV1.K2_GetRandomLocationInNavigableRadius` (`self.K2_GetActorLocation`) 10.0 null null)) "Undefined" "OverrideRootScale" null (`|GetArrayItem` _outrownames (`KismetMathLibrary.RandomInteger` (`KismetArrayLibrary.Array_Length` _outrownames))) "Weapon1" null)))))

(fn `UserConstructionScript`)