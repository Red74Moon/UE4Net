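; BP_Durmy is a moving actor that updates the score and disappears when the player character touches it.
; A looping timer calls MoveFront every hundredth of a second to shift the Cube component along its relative Y axis, scaled by Speed.
; When the Cube overlaps a ThirdPersonCharacter, it logs the hit, calls SetScoreText on the PlayHUD and destroys the actor.
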(event `self.ReceiveBeginPlay`
  (`KismetSystemLibrary.K2_SetTimer` null "MoveFront" 0.01 true))

(event `self.Cube.OnComponentBeginOverlap`
  (params (OverlappedComponent :type "PrimitiveComponent Object Reference") (OtherActor :type "Actor Object Reference") (OtherComp :type "PrimitiveComponent Object Reference") (OtherBodyIndex :type Integer) (bFromSweep :type Boolean) (SweepResult :type "HitResult Structure (by ref)"))
  (cast `/Game/ThirdPersonBP/Blueprints/ThirdPersonCharacter` OtherActor)
  (`KismetSystemLibrary.PrintString` "Durmy OverLap" false true (struct :`G` 0.66 :`B` 1.0 :`A` 1.0) 20.0)
  (bind _asplay_hud (cast `/Game/Durmy/Play/PlayHUD` (`PlayerController.GetHUD` (`GameplayStatics.GetPlayerController` 0))))
  (`/Game/Durmy/Play/PlayHUD.SetScoreText` _asplay_hud)
  (`self.K2_DestroyActor` self))

(fn `MoveFront`
  (`SceneComponent.K2_AddRelativeLocation` (`self.Cube`) (`KismetMathLibrary.MakeVector` 0.0 (* (`self.Speed`) 0.01)) false false))

(fn `UserConstructionScript`)