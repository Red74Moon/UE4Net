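; BP_Spawn is a spawner that keeps creating BP_Durmy actors during play.
; On BeginPlay it starts a looping one-second timer that calls SpawnActor by function name.
; Each call spawns a BP_Durmy at a random X and Z within set ranges on a fixed Y, then tells the first player's PlayHUD to update its total text.
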(event `self.ReceiveBeginPlay`
  (`|ExecutionSequence`
    (:`then_0`
      (`self.DoSpawnActor`))))

(fn `DoSpawnActor`
  (`KismetSystemLibrary.K2_SetTimer` null "SpawnActor" 1.0 true))

(fn `SpawnActor`
  (`|SpawnActorFromClass` "/Game/Durmy/Play/BP_Durmy.BP_Durmy_C" (`KismetMathLibrary.MakeTransform` (`KismetMathLibrary.MakeVector` (`KismetMathLibrary.RandomFloatInRange` -700.0 -1200.0) -840.0 (`KismetMathLibrary.RandomFloatInRange` 150.0 350.0))) "Undefined" "OverrideRootScale" null null)
  (bind _asplay_hud (cast `/Game/Durmy/Play/PlayHUD` (`PlayerController.GetHUD` (`GameplayStatics.GetPlayerController` 0))))
  (`/Game/Durmy/Play/PlayHUD.SetTotalText` _asplay_hud))

(fn `UserConstructionScript`)