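; BP_PlayGameInstance is a game instance Blueprint that holds the play score, a date-time value and a list of score records.
; Setter and getter functions handle the score and date-time.
; AddArray joins both values into a "::"-separated string, inserts it into ScoreArray at a running index, then advances that index when the array length exceeds it.
; ShowArray prints each stored record for inspection.
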(fn `AddArray`
  (`KismetArrayLibrary.Array_Insert` (`self.ScoreArray`) (`KismetStringLibrary.Concat_StrStr` (`self.DateTime`) " :: " (`KismetStringLibrary.Conv_IntToString` (`self.Score`))) (`self.IndexArray`))
  (if (> (`KismetArrayLibrary.Array_Length` (`self.ScoreArray`)) (`self.IndexArray`))
    (bind _result (`/Engine/EditorBlueprintResources/StandardMacros.IncrementInt` (`self.IndexArray`))
      (:`  `
        (set `self.IndexArray` _result)))))

(fn `GetDateTime`
  (returns (DateTime :type String))
  (return (`self.DateTime`)))

(fn `GetScore`
  (set `self.Score` (`self.Score`)))

(fn `SetDateTime`
  (params (DateTime :type String))
  (set `self.DateTime` DateTime))

(fn `SetScore`
  (params (Score :type Integer))
  (set `self.Score` Score))

(fn `ShowArray`
  (for _index (range (+ (`KismetArrayLibrary.Array_Length` (`self.ScoreArray`)) 1))
    (`KismetSystemLibrary.PrintString` (`KismetStringLibrary.Concat_StrStr` "Array에 저장된 값 :: " (`|GetArrayItem` (`self.ScoreArray`) _index)))))