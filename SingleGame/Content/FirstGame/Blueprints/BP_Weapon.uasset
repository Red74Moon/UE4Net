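; BP_Weapon is a weapon actor that can be attached to or detached from a character and drives an on-screen pickup guide.
; ShowPickUpGuide starts a fast looping timer that passes the actor's location to BP_SingleHUD, until PickUpCollision's end overlap clears it.
; AttachToChar disables the static mesh's physics and collision and snaps it to a named socket on the character mesh.
; DetachToChar restores both and releases the mesh in place.
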(event `/Game/FirstGame/Data/BPI_PickUp.ShowPickUpGuide`
  (`KismetSystemLibrary.K2_SetTimer` null "UpdatePickupGuide" 0.01 true))

(event `self.PickUpCollision.OnComponentEndOverlap`
  (params (OverlappedComponent :type "PrimitiveComponent Object Reference") (OtherActor :type "Actor Object Reference") (OtherComp :type "PrimitiveComponent Object Reference") (OtherBodyIndex :type Integer))
  (`KismetSystemLibrary.K2_ClearTimer` null "UpdatePickupGuide"))

(fn `AttachToChar`
  (params (Character :type "Character Object Reference"))
  (returns (Result :type Boolean))
  (bind _staticmesh (`self.StaticMesh`))
  (`PrimitiveComponent.SetSimulatePhysics` _staticmesh false)
  (`PrimitiveComponent.SetCollisionEnabled` _staticmesh "NoCollision")
  (bind _returnvalue (`SceneComponent.K2_AttachToComponent` _staticmesh (`Character.Mesh` Character) (`self.Socket Name`) "SnapToTarget" "SnapToTarget" "KeepWorld" true))
  (return _returnvalue))

(fn `DetachToChar`
  (params (Character :type "Character Object Reference"))
  (returns (Result :type Boolean))
  (bind _staticmesh (`self.StaticMesh`))
  (`PrimitiveComponent.SetCollisionEnabled` _staticmesh "QueryAndPhysics")
  (`PrimitiveComponent.SetSimulatePhysics` _staticmesh true)
  (`SceneComponent.K2_DetachFromComponent` _staticmesh "KeepWorld" "KeepWorld" "KeepWorld" true)
  (return true))

(fn `UpdatePickupGuide`
  (bind _asbp_single_hud (cast `/Game/FirstGame/GameMode/BP_SingleHUD` (`PlayerController.GetHUD` (`GameplayStatics.GetPlayerController` 0))))
  (`/Game/FirstGame/GameMode/BP_SingleHUD.UpdatePickUpGuidePosition` _asbp_single_hud (`self.K2_GetActorLocation`)))

(fn `UserConstructionScript`)