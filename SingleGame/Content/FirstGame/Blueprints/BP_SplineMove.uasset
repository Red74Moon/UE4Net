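; Actor that moves a Cube back and forth along its Spline at a set Speed, ping-ponging between both ends.
; Tick calls MoveForward or MoveBackward based on IsFoward; each advances Distance, places the cube at that spline point's local location and rotation, and flips the flag at the ends.
; An unconnected Timeline holds an alternative spline-movement setup that never runs.
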(event `self.ReceiveTick`
  (params (DeltaSeconds :type "Float (single-precision)"))
  (if (`self.IsFoward`)
    (`self.MoveForward` DeltaSeconds)
    (else
      (`self.MoveBackward` DeltaSeconds))))

(fn `MoveBackward`
  (params (DeltaSecond :type "Float (double-precision)"))
  (bind _spline (`self.Spline`))
  (bind _cube (`self.Cube`))
  (bind _output_get (set `self.Distance` (- (`self.Distance`) (* DeltaSecond (`self.Speed`)))))
  (`SceneComponent.K2_SetRelativeTransform` _cube (`KismetMathLibrary.MakeTransform` (`SplineComponent.GetLocationAtDistanceAlongSpline` _spline _output_get "Local") (`SplineComponent.GetRotationAtDistanceAlongSpline` _spline _output_get "Local") (`SceneComponent.RelativeScale3D` _cube)) false false)
  (if (<= (`self.Distance`) 0.0)
    (set `self.IsFoward` true)))

(fn `MoveForward`
  (params (DeltaSecond :type "Float (double-precision)"))
  (bind _cube (`self.Cube`))
  (bind _spline (`self.Spline`))
  (bind _output_get (set `self.Distance` (+ (* DeltaSecond (`self.Speed`)) (`self.Distance`))))
  (`SceneComponent.K2_SetRelativeTransform` _cube (`KismetMathLibrary.MakeTransform` (`SplineComponent.GetLocationAtDistanceAlongSpline` _spline _output_get "Local") (`SplineComponent.GetRotationAtDistanceAlongSpline` _spline _output_get "Local") (`SceneComponent.RelativeScale3D` _cube)) false false)
  (if (> (`self.Distance`) (`SplineComponent.GetSplineLength` (`self.Spline`)))
    (set `self.IsFoward` false)))

(fn `UserConstructionScript`)