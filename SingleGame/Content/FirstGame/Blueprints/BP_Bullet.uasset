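; BP_Bullet is a homing projectile that locks onto player pawn 0 on spawn and ragdolls any BP_FirstCharacter it overlaps, then destroys itself.
; DoShoot aims the Sphere at the target and starts a looping timer on MoveForward, which gradually lerps rotation toward the target while advancing without sweep.
; MoveUFO (direct pursuit) and MoveBullet (straight flight) are alternative movement functions whose timers never run.
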(event `self.ReceiveBeginPlay`
  (`self.DoShoot` (`GameplayStatics.GetPlayerPawn` 0)))

(event `self.Sphere.OnComponentBeginOverlap`
  (params (OverlappedComponent :type "PrimitiveComponent Object Reference") (OtherActor :type "Actor Object Reference") (OtherComp :type "PrimitiveComponent Object Reference") (OtherBodyIndex :type Integer) (bFromSweep :type Boolean) (SweepResult :type "HitResult Structure (by ref)"))
  (`KismetSystemLibrary.PrintString` (`KismetSystemLibrary.GetDisplayName` OtherActor))
  (bind _asbp_first_character (cast `/Game/FirstGame/GameMode/BP_FirstCharacter` OtherActor))
  (`/Game/FirstGame/GameMode/BP_FirstCharacter.DoRagdoll` _asbp_first_character)
  (`KismetSystemLibrary.K2_ClearTimer` null "MoveForward")
  (`self.K2_DestroyActor`))

(fn `DoShoot`
  (params (Target :type "Actor Object Reference"))
  (bind _sphere (`self.Sphere`))
  (set `self.Target` Target)
  (`SceneComponent.K2_SetWorldRotation` _sphere (`KismetMathLibrary.FindLookAtRotation` (`SceneComponent.K2_GetComponentLocation` _sphere) (`self.K2_GetActorLocation` (`self.Target`))) false false)
  (`KismetSystemLibrary.K2_SetTimer` null "MoveForward" 0.01 true))

(fn `MoveBullet`
  (bind _sphere (`self.Sphere`))
  (`/Engine/EditorBlueprintResources/StandardMacros.IsValid` (`self.Target`)
    (:`Is Valid`
      (`SceneComponent.K2_AddWorldOffset` _sphere (* (`SceneComponent.GetForwardVector` _sphere) (* 0.01 (`self.Speed`))) false false))
    (:`Is Not Valid`
      (`KismetSystemLibrary.PrintString` "Target is nullptr"))))

(fn `MoveForward`
  (bind _sphere (`self.Sphere`))
  (bind _sphere_2 (`self.Sphere`))
  (`/Engine/EditorBlueprintResources/StandardMacros.IsValid` (`self.Target`)
    (:`Is Valid`
      (`SceneComponent.K2_SetWorldRotation` _sphere (`KismetMathLibrary.RLerp` (`SceneComponent.K2_GetComponentRotation` _sphere) (`KismetMathLibrary.FindLookAtRotation` (`SceneComponent.K2_GetComponentLocation` (`self.Sphere`)) (`self.K2_GetActorLocation` (`self.Target`))) 0.01 true) false false)
      (`SceneComponent.K2_AddWorldOffset` _sphere_2 (* (`SceneComponent.GetForwardVector` _sphere_2) (* 0.01 (`self.Speed`))) false false))
    (:`Is Not Valid`
      (`KismetSystemLibrary.PrintString` "Target is nullptr"))))

(fn `MoveUFO`
  (`/Engine/EditorBlueprintResources/StandardMacros.IsValid` (`self.Target`)
    (:`Is Valid`
      (`SceneComponent.K2_AddWorldOffset` (`self.Sphere`) (* (`KismetMathLibrary.GetForwardVector` (`KismetMathLibrary.FindLookAtRotation` (`SceneComponent.K2_GetComponentLocation` (`self.Sphere`)) (`self.K2_GetActorLocation` (`self.Target`)))) (* 0.01 (`self.Speed`))) false false))
    (:`Is Not Valid`
      (`KismetSystemLibrary.PrintString` "Target is nullptr"))))

(fn `UserConstructionScript`)