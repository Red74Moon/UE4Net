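; Player character for a jump game that handles camera-relative movement, look and jump, and opens the JumpHud pause box on P.
; On server Tick it pushes its height, derived from world Z scaled to meters, to JumpPlayerState through UpdateHeight.
; A separate ReqHeight/ResHeight path sets the height with debug prints, but the timer setup meant to drive it is disconnected.
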(event `InputAxis|Turn`
  (params (AxisValue :type "Float (single-precision)"))
  ;[1 1 1] 케릭터 움직임
  (`self.AddControllerYawInput` AxisValue))

(event `InputAction|Jump`
  (params (Key :type "Key Structure"))
  (:`Pressed`
    (`self.Jump`)
    (`KismetSystemLibrary.PrintString` "Jump 실행" false true (struct :`G` 0.66 :`B` 1.0 :`A` 1.0) 20.0))
  (:`Released`
    (`self.StopJumping`)))

(event `InputAxis|LookUp`
  (params (AxisValue :type "Float (single-precision)"))
  ;[1 1 1] 케릭터 움직임
  (`self.AddControllerPitchInput` AxisValue))

(event `InputAxis|MoveForward`
  (params (AxisValue :type "Float (single-precision)"))
  (bind (_returnvalue_x _returnvalue_y) (`KismetMathLibrary.BreakVector` (`self.GetActorForwardVector` (`GameplayStatics.GetPlayerCameraManager` 0))))
  ;[1 1 1] 케릭터 움직임
  (`self.AddMovementInput` (`KismetMathLibrary.MakeVector` _returnvalue_x _returnvalue_y) AxisValue))

(event `InputAxis|MoveRight`
  (params (AxisValue :type "Float (single-precision)"))
  (bind (_returnvalue_x _returnvalue_y) (`KismetMathLibrary.BreakVector` (`self.GetActorRightVector` (`GameplayStatics.GetPlayerCameraManager` 0))))
  ;[1 1 1] 케릭터 움직임
  (`self.AddMovementInput` (`KismetMathLibrary.MakeVector` _returnvalue_x _returnvalue_y) AxisValue))

(event `self.ReceiveTick`
  (params (DeltaSeconds :type "Float (single-precision)"))
  (`/Engine/EditorBlueprintResources/ActorMacros.Switch Has Authority`
    (:`Authority`
      (bind _asjump_player_state (cast `/Game/Learn_Collision/HUD/Game/JumpPlayerState` (`self.PlayerState`)))
      (`/Game/Learn_Collision/HUD/Game/JumpPlayerState.UpdateHeight` _asjump_player_state (`self.GetHeight`)))))

(event `Key|P`
  (params (Key :type "Key Structure"))
  (:`Pressed`
    (bind _asjump_hud (cast `/Game/Learn_Collision/HUD/Game/JumpHud` (`PlayerController.GetHUD` (`GameplayStatics.GetPlayerController` 0))))
    (`/Game/Learn_Collision/HUD/Game/JumpHud.ShowPauseBox` _asjump_hud)))

(event `self.ReceiveBeginPlay`)

(event `ReqHeight`
  ;[1 0 0] (서버)
  (`KismetSystemLibrary.PrintString` "ReqHeight 요청" true true (struct :`G` 0.66 :`B` 1.0 :`A` 1.0) 20.0)
  (`self.ResHeight`))

(event `ResHeight`
  (bind _resultheight (`self.GetHeight`))
  (`KismetSystemLibrary.PrintString` "ResHeight 요청" true true (struct :`G` 0.66 :`B` 1.0 :`A` 1.0) 20.0)
  (bind _asjump_player_state (cast `/Game/Learn_Collision/HUD/Game/JumpPlayerState` (`self.PlayerState`)))
  (`/Game/Learn_Collision/HUD/Game/JumpPlayerState.SetHeight` _asjump_player_state _resultheight)
  (`KismetSystemLibrary.PrintString` (`KismetStringLibrary.Concat_StrStr` "server 에서 입력되는 Height : " (`KismetStringLibrary.Conv_IntToString` _resultheight)) true true (struct :`G` 0.66 :`B` 1.0 :`A` 1.0) 20.0))

(fn `GetHeight`
  (returns (ResultHeight :type Integer))
  (bind (_returnvalue_x _returnvalue_y _returnvalue_z) (`KismetMathLibrary.BreakVector` (`self.K2_GetActorLocation` self)))
  (return (/ (`KismetMathLibrary.FFloor` _returnvalue_z) 100)))

(fn `ReqCall`
  (`self.ReqHeight`))

(fn `SetHeight`
  (params (Height :type Integer))
  (set `self.Height` Height))

(fn `UserConstructionScript`)