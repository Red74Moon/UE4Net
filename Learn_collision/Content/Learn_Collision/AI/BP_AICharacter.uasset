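; BP_AICharacter is a character Blueprint that handles basic player locomotion through legacy input axis and action mappings; despite its name, it contains no AI logic.
; Turn and look axes drive controller yaw and pitch, while the jump action starts and stops jumping.
; Forward and right movement follow player 0's camera manager vectors, using only their X and Y components without renormalizing.
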(event `InputAxis|Turn`
  (params (AxisValue :type "Float (single-precision)"))
  ;[1 1 1] 케릭터 움직임
  (`self.AddControllerYawInput` AxisValue))

(event `InputAction|Jump`
  (params (Key :type "Key Structure"))
  ;[1 1 1] 케릭터 움직임
  (:`Pressed`
    (`self.Jump`))
  (:`Released`
    (`self.StopJumping`)))

(event `InputAxis|LookUp`
  (params (AxisValue :type "Float (single-precision)"))
  ;[1 1 1] 케릭터 움직임
  (`self.AddControllerPitchInput` AxisValue))

(event `InputAxis|MoveForward`
  (params (AxisValue :type "Float (single-precision)"))
  (bind (_returnvalue_x _returnvalue_y) (`KismetMathLibrary.BreakVector` (`self.GetActorForwardVector` (`GameplayStatics.GetPlayerCameraManager` 0))))
  ;[1 1 1] 케릭터 움직임
  (`self.AddMovementInput` (`KismetMathLibrary.MakeVector` _returnvalue_x _returnvalue_y) AxisValue))

(event `InputAxis|MoveRight`
  (params (AxisValue :type "Float (single-precision)"))
  (bind (_returnvalue_x _returnvalue_y) (`KismetMathLibrary.BreakVector` (`self.GetActorRightVector` (`GameplayStatics.GetPlayerCameraManager` 0))))
  ;[1 1 1] 케릭터 움직임
  (`self.AddMovementInput` (`KismetMathLibrary.MakeVector` _returnvalue_x _returnvalue_y) AxisValue))

(fn `UserConstructionScript`)