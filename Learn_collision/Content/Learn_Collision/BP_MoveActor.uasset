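; Practice actor that slides its Sphere component back and forth along local X while IsPlay is true.
; Tick calls MoveSphere, which offsets the sphere by delta time and flips IsMove at the 0 and 200 bounds.
; PressP is empty, with its IsPlay toggle left unconnected.
; MoveUp, MoveDown and CountTimer, a minutes/seconds printer fed by IntToStr00 zero-padding, are defined but never called here.
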(event `self.ReceiveTick`
  (params (DeltaSeconds :type "Float (single-precision)"))
  (if (`self.IsPlay`)
    (`self.MoveSphere` DeltaSeconds)))

(event `/Game/Learn_Collision/BPI_PressP.PressP`)

(fn `CountTimer`
  (params (DeltaSecond :type "Float (double-precision)"))
  (bind _output_get (set `self.TotalDest` (+ (* DeltaSecond 100.0) (`self.TotalDest`))))
  (bind _returnvalue (`KismetStringLibrary.Concat_StrStr` "" "" (`self.IntToStr00` (`KismetMathLibrary.FFloor` (/ _output_get 60.0))) "m" (`self.IntToStr00` (`KismetMathLibrary.FFloor` (mod _output_get 60.0))) "s"))
  (if (not (`KismetStringLibrary.EqualEqual_StrStr` (`self.OldTime`) _returnvalue))
    (`KismetSystemLibrary.PrintString` _returnvalue)
    (set `self.OldTime` _returnvalue)))

(fn `IntToStr00`
  (params (Time :type Integer))
  (returns (NewTime :type String))
  (if (< Time 10)
    (return (`KismetStringLibrary.Concat_StrStr` "0" (`KismetStringLibrary.Conv_IntToString` Time)))
    (else
      (return (`KismetStringLibrary.Conv_IntToString` Time)))))

(fn `MoveDown`
  (params (DeltaSecond :type "Float (double-precision)"))
  (bind _result (`/Engine/EditorBlueprintResources/StandardMacros.NegateFloat` (* DeltaSecond 100.0))
    (:`  `
      (`SceneComponent.K2_AddLocalOffset` (`self.Sphere`) (`KismetMathLibrary.MakeVector` 0.0 0.0 _result) false false))))

(fn `MoveSphere`
  (params (A :type "Float (double-precision)"))
  (bind _returnvalue (* A 200.0))
  (bind _sphere (`self.Sphere`))
  (bind _relativelocation_x (`KismetMathLibrary.BreakVector` (`SceneComponent.RelativeLocation` (`self.Sphere`))))
  (bind _relativelocation_x_2 (`KismetMathLibrary.BreakVector` (`SceneComponent.RelativeLocation` (`self.Sphere`))))
  (if (`self.IsPlay`)
    (if (`self.IsMove`)
      (`SceneComponent.K2_AddLocalOffset` _sphere (`KismetMathLibrary.MakeVector` _returnvalue) false false)
      (if (> _relativelocation_x 200.0)
        (set `self.IsMove` false))
      (else
        (bind _result (`/Engine/EditorBlueprintResources/StandardMacros.NegateFloat` _returnvalue)
          (:`  `
            (`SceneComponent.K2_AddLocalOffset` _sphere (`KismetMathLibrary.MakeVector` _result) false false)
            (if (< _relativelocation_x_2 0.0)
              (set `self.IsMove` true))))))))

(fn `MoveUp`
  (params (DeltaSecond :type "Float (double-precision)"))
  (bind _returnvalue (* DeltaSecond 100.0))
  (bind _sphere (`self.Sphere`))
  (bind (_relativelocation_x _relativelocation_y _relativelocation_z) (`KismetMathLibrary.BreakVector` (`SceneComponent.RelativeLocation` (`self.Sphere`))))
  (bind (_relativelocation_x_2 _relativelocation_y_2 _relativelocation_z_2) (`KismetMathLibrary.BreakVector` (`SceneComponent.RelativeLocation` (`self.Sphere`))))
  (if (`self.IsMove`)
    (bind _result (`/Engine/EditorBlueprintResources/StandardMacros.NegateFloat` _returnvalue)
      (:`  `
        (`SceneComponent.K2_AddLocalOffset` _sphere (`KismetMathLibrary.MakeVector` 0.0 0.0 _returnvalue) false false)
        (if (> _relativelocation_z_2 200.0)
          (set `self.IsMove` false))))
    (else
      (`SceneComponent.K2_AddLocalOffset` _sphere (`KismetMathLibrary.MakeVector` 0.0 0.0 _result) false false)
      (if (<= _relativelocation_z 0.0)
        (set `self.IsMove` true)))))

(fn `UserConstructionScript`)