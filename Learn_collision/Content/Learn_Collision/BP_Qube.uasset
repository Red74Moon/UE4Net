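; BP_Qube is a collision-practice cube actor that swaps its material and runs a timer while something overlaps it.
; Overlap begin and end toggle a flag that lets Tick call CountTime, which accumulates delta time at 100x speed into a persistent total.
; When the zero-padded minutes/seconds string from IntToStr00 changes, it prints the new time and nudges the actor along local X by a delta-scaled step.
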(event `self.ReceiveTick`
  (params (DeltaSeconds :type "Float (single-precision)"))
  (if (`self.IsCountTime`)
    (`self.CountTime` DeltaSeconds)))

(event `self.Cube.OnComponentBeginOverlap`
  (params (OverlappedComponent :type "PrimitiveComponent Object Reference") (OtherActor :type "Actor Object Reference") (OtherComp :type "PrimitiveComponent Object Reference") (OtherBodyIndex :type Integer) (bFromSweep :type Boolean) (SweepResult :type "HitResult Structure (by ref)"))
  (set `self.IsCountTime` true)
  (`PrimitiveComponent.SetMaterial` (`self.Cube`) 0 "/Game/Geometry/Meshes/CubeMaterial.CubeMaterial"))

(event `self.Cube.OnComponentEndOverlap`
  (params (OverlappedComponent :type "PrimitiveComponent Object Reference") (OtherActor :type "Actor Object Reference") (OtherComp :type "PrimitiveComponent Object Reference") (OtherBodyIndex :type Integer))
  (set `self.IsCountTime` false)
  (`PrimitiveComponent.SetMaterial` (`self.Cube`) 0 "/Game/StarterContent/Materials/M_CobbleStone_Pebble.M_CobbleStone_Pebble"))

(fn `CountTime`
  (params (DeltaSecond :type "Float (double-precision)"))
  (bind _returnvalue (* DeltaSecond 100.0))
  (bind _output_get (set `self.Total Dest` (+ _returnvalue (`self.Total Dest`))))
  (bind _returnvalue_2 (`KismetStringLibrary.Concat_StrStr` "" "" (`self.IntToStr00` (`KismetMathLibrary.FFloor` (/ _output_get 60.0))) "m" (`self.IntToStr00` (`KismetMathLibrary.FFloor` (mod _output_get 60.0))) "s"))
  (if (not (`KismetStringLibrary.EqualEqual_StrStr` (`self.Old Time`) _returnvalue_2))
    (`KismetSystemLibrary.PrintString` _returnvalue_2)
    (set `self.Old Time` _returnvalue_2)
    (`self.K2_AddActorLocalOffset` (`KismetMathLibrary.MakeVector` _returnvalue))))

(fn `IntToStr00`
  (params (Time :type Integer))
  (returns (NewTime :type String))
  (if (< Time 10)
    (return (`KismetStringLibrary.Concat_StrStr` "0" (`KismetStringLibrary.Conv_IntToString` Time)))
    (else
      (return (`KismetStringLibrary.Conv_IntToString` Time)))))

(fn `UserConstructionScript`)