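; BP_SchoolBell plays a school bell melody automatically on BeginPlay, displaying each pitch on a text render.
; BeatTimer reads the current row of DT_SchoolBell, then uses its pitch name to look up and play the matching DT_Piano sound.
; It re-arms itself by timer with that note's beat as the delay, stopping once the index passes a hardcoded 24.
; ShowPitchText also prints the index and pitch for debugging.
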(event `self.ReceiveBeginPlay`
  (`self.BeatTimer`))

(fn `BeatTimer`
  (bind _index (`self.Index`))
  (if (not (> _index 24))
    (bind _returnvalue (`|GetDataTableRow` "/Game/Piano/Song/DT_SchoolBell.DT_SchoolBell" (`KismetStringLibrary.Conv_StringToName` (`KismetStringLibrary.Conv_IntToString` _index)))
      (:`then`
        (bind (_pitch _pitchname _beat) (break `/Game/Piano/Song/ST_Song` _returnvalue))
        (bind _returnvalue_2 (`|GetDataTableRow` "/Game/Piano/DT_Piano.DT_Piano" (`KismetStringLibrary.Conv_StringToName` (`KismetTextLibrary.Conv_TextToString` _pitchname)))
          (:`then`
            (`GameplayStatics.PlaySound2D` (`.Sound_12_985E51EF4C9F77B2743A2283419A888F` (break `/Game/Piano/ST_Piano` _returnvalue_2)) 1.0 1.0 0.0 null null)
            (`self.ShowPitchText`)
            (`/Engine/EditorBlueprintResources/StandardMacros.IncrementInt` (`self.Index`)
              (:`  `
                (`KismetSystemLibrary.K2_SetTimer` null "BeatTimer" _beat))))
          (:`RowNotFound`
            (`KismetSystemLibrary.PrintString` "DT_Piano RowName Not Found!" true true (struct :`R` 1.0 :`A` 1.0) 20.0)))))))

(fn `ShowPitchText`
  (bind _index (`self.Index`))
  (if (not (> _index 24))
    (`KismetSystemLibrary.PrintString` (`KismetStringLibrary.Concat_StrStr` "index : " (`KismetStringLibrary.Conv_IntToString` _index)) true true (struct :`G` 0.66 :`B` 1.0 :`A` 1.0) 20.0)
    (bind _returnvalue (`DataTableFunctionLibrary.GetDataTableColumnAsString` "/Game/Piano/Song/DT_SchoolBell.DT_SchoolBell" "Pitch"))
    (bind _output (`|GetArrayItem` _returnvalue (- (`self.Index`) 1)))
    (`KismetSystemLibrary.PrintString` _output true true (struct :`G` 0.66 :`B` 1.0 :`A` 1.0) 20.0)
    (`TextRenderComponent.K2_SetText` (`self.TextRender`) (`KismetTextLibrary.Conv_StringToText` _output))))

(fn `UserConstructionScript`)