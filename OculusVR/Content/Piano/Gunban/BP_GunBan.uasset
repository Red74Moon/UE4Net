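; BP_GunBan is a piano key actor that plays its note when something overlaps its Cube.
; The overlap looks up RowName in DT_Piano, plays that row's sound in 2D and passes its pitch name to the Name text.
; A half-second timer hides the text again.
; A separate color-change function turns the Cube green for pitch G, and an unconnected BP_SchoolBell dispatcher binding never runs.
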(event `self.ReceiveBeginPlay`)

(event `self.Cube.OnComponentBeginOverlap`
  (params (OverlappedComponent :type "PrimitiveComponent Object Reference") (OtherActor :type "Actor Object Reference") (OtherComp :type "PrimitiveComponent Object Reference") (OtherBodyIndex :type Integer) (bFromSweep :type Boolean) (SweepResult :type "HitResult Structure (by ref)"))
  (`KismetSystemLibrary.PrintString` "Touch GunBan" false true (struct :`G` 0.66 :`B` 1.0 :`A` 1.0) 60.0)
  (`self.PlaySound`))

(fn `BP_GunBan_ColorChange`
  (params (Pitch :type "/Game/Piano/Gunban/EN_Piano Enum" :default "NewEnumerator0"))
  (switch `/Game/Piano/Gunban/EN_Piano` Pitch
    (:`NewEnumerator7`
      (`PrimitiveComponent.SetMaterial` (`self.Cube`) 0 "/AnimationSharing/AnimSharingGreen.AnimSharingGreen"))))

(fn `ClearGunbanText`
  (`SceneComponent.SetVisibility` (`self.Name`) false false))

(fn `PlaySound`
  (`ActorComponent.SetAutoActivate` (`self.Audio`) true)
  (bind _returnvalue (`|GetDataTableRow` "/Game/Piano/Gunban/DT_Piano.DT_Piano" (`self.Row Name`))
    (:`then`
      (bind (_pitch _pitchname _sound) (break `/Game/Piano/Gunban/ST_Piano` _returnvalue))
      (`self.ShowSoundName` _pitchname)
      (`GameplayStatics.PlaySound2D` _sound 1.0 1.0 0.0 null null))))

(fn `ShowSoundName`
  (params (PitchName :type "Text (by ref)"))
  (bind _name (`self.Name`))
  (`SceneComponent.SetVisibility` _name true false)
  (`TextRenderComponent.K2_SetText` _name PitchName)
  (`KismetSystemLibrary.K2_SetTimer` null "ClearGunbanText" 0.5))

(fn `UserConstructionScript`)