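; BP_Xylophone is a playable xylophone with a collision box for each note from C through B, plus C4.
; On BeginPlay, SlientSound turns off auto-activate on every note's audio component.
; Each box overlap re-enables auto-activate (C4 toggles BAudio) and spawns that note's sound from its DT_Piano row.
; D and E play as 2D sounds, while the other notes spawn at world origin.
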(event `self.ReceiveBeginPlay`
  (`self.SlientSound`))

(event `self.C_BoxCol.OnComponentBeginOverlap`
  (params (OverlappedComponent :type "PrimitiveComponent Object Reference") (OtherActor :type "Actor Object Reference") (OtherComp :type "PrimitiveComponent Object Reference") (OtherBodyIndex :type Integer) (bFromSweep :type Boolean) (SweepResult :type "HitResult Structure (by ref)"))
  (`ActorComponent.SetAutoActivate` (`self.C_Audio`) true)
  (bind _returnvalue (`|GetDataTableRow` "/Game/Piano/Gunban/DT_Piano.DT_Piano" "C")
    (:`then`
      (`GameplayStatics.SpawnSoundAtLocation` (`.Sound_12_985E51EF4C9F77B2743A2283419A888F` (break `/Game/Piano/Gunban/ST_Piano` _returnvalue)) (0.0 0.0 0.0) (struct) 1.0 1.0 0.0 null null))))

(event `self.D_BoxCol.OnComponentBeginOverlap`
  (params (OverlappedComponent :type "PrimitiveComponent Object Reference") (OtherActor :type "Actor Object Reference") (OtherComp :type "PrimitiveComponent Object Reference") (OtherBodyIndex :type Integer) (bFromSweep :type Boolean) (SweepResult :type "HitResult Structure (by ref)"))
  (`ActorComponent.SetAutoActivate` (`self.D_Audio`) true)
  (bind _returnvalue (`|GetDataTableRow` "/Game/Piano/Gunban/DT_Piano.DT_Piano" "D")
    (:`then`
      (`GameplayStatics.SpawnSound2D` (`.Sound_12_985E51EF4C9F77B2743A2283419A888F` (break `/Game/Piano/Gunban/ST_Piano` _returnvalue)) 1.0 1.0 0.0 null))))

(event `self.E_BoxCol.OnComponentBeginOverlap`
  (params (OverlappedComponent :type "PrimitiveComponent Object Reference") (OtherActor :type "Actor Object Reference") (OtherComp :type "PrimitiveComponent Object Reference") (OtherBodyIndex :type Integer) (bFromSweep :type Boolean) (SweepResult :type "HitResult Structure (by ref)"))
  (`ActorComponent.SetAutoActivate` (`self.E_Audio`) true)
  (bind _returnvalue (`|GetDataTableRow` "/Game/Piano/Gunban/DT_Piano.DT_Piano" "E")
    (:`then`
      (`GameplayStatics.SpawnSound2D` (`.Sound_12_985E51EF4C9F77B2743A2283419A888F` (break `/Game/Piano/Gunban/ST_Piano` _returnvalue)) 1.0 1.0 0.0 null))))

(event `self.F_BoxCol.OnComponentBeginOverlap`
  (params (OverlappedComponent :type "PrimitiveComponent Object Reference") (OtherActor :type "Actor Object Reference") (OtherComp :type "PrimitiveComponent Object Reference") (OtherBodyIndex :type Integer) (bFromSweep :type Boolean) (SweepResult :type "HitResult Structure (by ref)"))
  (`ActorComponent.SetAutoActivate` (`self.F_Audio`) true)
  (bind _returnvalue (`|GetDataTableRow` "/Game/Piano/Gunban/DT_Piano.DT_Piano" "F")
    (:`then`
      (`GameplayStatics.SpawnSoundAtLocation` (`.Sound_12_985E51EF4C9F77B2743A2283419A888F` (break `/Game/Piano/Gunban/ST_Piano` _returnvalue)) (0.0 0.0 0.0) (struct) 1.0 1.0 0.0 null null))))

(event `self.G_BoxCol.OnComponentBeginOverlap`
  (params (OverlappedComponent :type "PrimitiveComponent Object Reference") (OtherActor :type "Actor Object Reference") (OtherComp :type "PrimitiveComponent Object Reference") (OtherBodyIndex :type Integer) (bFromSweep :type Boolean) (SweepResult :type "HitResult Structure (by ref)"))
  (`ActorComponent.SetAutoActivate` (`self.G_Audio`) true)
  (bind _returnvalue (`|GetDataTableRow` "/Game/Piano/Gunban/DT_Piano.DT_Piano" "G")
    (:`then`
      (`GameplayStatics.SpawnSoundAtLocation` (`.Sound_12_985E51EF4C9F77B2743A2283419A888F` (break `/Game/Piano/Gunban/ST_Piano` _returnvalue)) (0.0 0.0 0.0) (struct) 1.0 1.0 0.0 null null))))

(event `self.A_BoxCol.OnComponentBeginOverlap`
  (params (OverlappedComponent :type "PrimitiveComponent Object Reference") (OtherActor :type "Actor Object Reference") (OtherComp :type "PrimitiveComponent Object Reference") (OtherBodyIndex :type Integer) (bFromSweep :type Boolean) (SweepResult :type "HitResult Structure (by ref)"))
  (`ActorComponent.SetAutoActivate` (`self.A_Audio`) true)
  (bind _returnvalue (`|GetDataTableRow` "/Game/Piano/Gunban/DT_Piano.DT_Piano" "A")
    (:`then`
      (`GameplayStatics.SpawnSoundAtLocation` (`.Sound_12_985E51EF4C9F77B2743A2283419A888F` (break `/Game/Piano/Gunban/ST_Piano` _returnvalue)) (0.0 0.0 0.0) (struct) 1.0 1.0 0.0 null null))))

(event `self.B_BoxCol.OnComponentBeginOverlap`
  (params (OverlappedComponent :type "PrimitiveComponent Object Reference") (OtherActor :type "Actor Object Reference") (OtherComp :type "PrimitiveComponent Object Reference") (OtherBodyIndex :type Integer) (bFromSweep :type Boolean) (SweepResult :type "HitResult Structure (by ref)"))
  (`ActorComponent.SetAutoActivate` (`self.B_Audio`) true)
  (bind _returnvalue (`|GetDataTableRow` "/Game/Piano/Gunban/DT_Piano.DT_Piano" "B")
    (:`then`
      (`GameplayStatics.SpawnSoundAtLocation` (`.Sound_12_985E51EF4C9F77B2743A2283419A888F` (break `/Game/Piano/Gunban/ST_Piano` _returnvalue)) (0.0 0.0 0.0) (struct) 1.0 1.0 0.0 null null))))

(event `self.C4_BoxCol.OnComponentBeginOverlap`
  (params (OverlappedComponent :type "PrimitiveComponent Object Reference") (OtherActor :type "Actor Object Reference") (OtherComp :type "PrimitiveComponent Object Reference") (OtherBodyIndex :type Integer) (bFromSweep :type Boolean) (SweepResult :type "HitResult Structure (by ref)"))
  (`ActorComponent.SetAutoActivate` (`self.B_Audio`) true)
  (bind _returnvalue (`|GetDataTableRow` "/Game/Piano/Gunban/DT_Piano.DT_Piano" "C4")
    (:`then`
      (`GameplayStatics.SpawnSoundAtLocation` (`.Sound_12_985E51EF4C9F77B2743A2283419A888F` (break `/Game/Piano/Gunban/ST_Piano` _returnvalue)) (0.0 0.0 0.0) (struct) 1.0 1.0 0.0 null null))))

(fn `SlientSound`
  (`ActorComponent.SetAutoActivate` (`self.C4_Audio`) false)
  (`ActorComponent.SetAutoActivate` (`self.C_Audio`) false)
  (`ActorComponent.SetAutoActivate` (`self.D_Audio`) false)
  (`ActorComponent.SetAutoActivate` (`self.E_Audio`) false)
  (`ActorComponent.SetAutoActivate` (`self.F_Audio`) false)
  (`ActorComponent.SetAutoActivate` (`self.G_Audio`) false)
  (`ActorComponent.SetAutoActivate` (`self.A_Audio`) false)
  (`ActorComponent.SetAutoActivate` (`self.B_Audio`) false))

(fn `UserConstructionScript`)